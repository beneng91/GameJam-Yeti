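; BP_Player is a prototype test player with debug keys, a pause screen and respawning.
; Keys toggle the BP_Yeti AI between passive and attacking this player, make an AI-audible noise with explosion effects, and print the key inventory.
; Escape adds a PauseScreen widget to the viewport.
; Death destroys the actor, and the Destroyed event asks BP_FirstPersonGameMode to respawn the player at the first BP_SpawnPoint found.
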(event `Key|One`
  (params (Key :type "Key Structure"))
  (:`Pressed`
    (bind _returnvalue (`GameplayStatics.GetActorOfClass` "/Game/Prototype/Test_Yeti/BP_Yeti.BP_Yeti_C"))
    (bind _asaic_yeti_base (cast `/Game/Prototype/Test_Yeti/AI/AIC_Yeti_Base` (`AIBlueprintHelperLibrary.GetAIController` _returnvalue)))
    (`/Engine/EditorBlueprintResources/StandardMacros.FlipFlop`
      (:`A`
        (`/Game/Prototype/Test_Yeti/AI/AIC_Yeti_Base.SetStateAsPassive` _asaic_yeti_base))
      (:`B`
        (`/Game/Prototype/Test_Yeti/AI/AIC_Yeti_Base.SetStateAsAttacking` _asaic_yeti_base self)))))

(event `Key|F`
  (params (Key :type "Key Structure"))
  (bind _returnvalue (`self.K2_GetActorLocation`))
  (:`Pressed`
    (`self.MakeNoise` 1.0 self _returnvalue)
    (`GameplayStatics.SpawnEmitterAtLocation` "/Game/StarterContent/Particles/P_Explosion.P_Explosion" _returnvalue)
    (`GameplayStatics.PlaySoundAtLocation` "/Game/StarterContent/Audio/Explosion_Cue.Explosion_Cue" _returnvalue (struct) 1.0 1.0 0.0 null null null null)))

(event `Key|R`
  (params (Key :type "Key Structure"))
  ;[1 1 1] Testing for Key
  (:`Pressed`
    (for _array_element (`self.KeyInventory`)
      (`KismetSystemLibrary.PrintString` (`KismetStringLibrary.Conv_IntToString` _array_element)))))

(event `Key|Escape`
  (params (Key :type "Key Structure"))
  ;[1 1 1] Pause Menu
  (:`Pressed`
    (bind _returnvalue (`|CreateWidget` "/Game/Prototype/UI/PauseMenu/PauseScreen.PauseScreen_C" (`GameplayStatics.GetPlayerController` 0)))
    (`UserWidget.AddToViewport` _returnvalue 0)))

(event `Death`
  ;[1 1 1] Death and Respawn
  (`self.K2_DestroyActor`))

(event `self.ReceiveDestroyed`
  ;[1 1 1] Death and Respawn
  (bind _outactors (`GameplayStatics.GetAllActorsOfClass` "/Game/Prototype/Test_Player/BP_SpawnPoint.BP_SpawnPoint_C"))
  (bind _asbp_first_person_game_mode (cast `/Game/FirstPerson/Blueprints/BP_FirstPersonGameMode` (`GameplayStatics.GetGameMode`)))
  (`/Game/FirstPerson/Blueprints/BP_FirstPersonGameMode.Respawn Player` _asbp_first_person_game_mode (`self.GetTransform` (`|GetArrayItem` _outactors))))

(fn `UserConstructionScript`)