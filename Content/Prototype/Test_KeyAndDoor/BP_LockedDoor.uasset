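; Prototype locked fence door that swings open when an overlapping BP_Player carries matching keys.
; On overlap it loops RequiredKeys, testing KeyInventory for both element and index; any single match sets IsOpen, despite the HasAllKeys name.
; Each miss prints debug text and the inventory.
; While IsOpen, Tick plays a Timeline that rotates FenceHinge's yaw, with a DoOnce-guarded opening sound.
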(event `self.ReceiveTick`
  (params (DeltaSeconds :type "Float (single-precision)"))
  (if (`self.IsOpen`)
    (bind (_direction _newtrack_0) (`Timeline|Timeline`)
      (:`Update`
        (`SceneComponent.K2_SetRelativeRotation` (`self.FenceHinge`) (`KismetMathLibrary.MakeRotator` 0.0 0.0 _newtrack_0) false false)
        (`/Engine/EditorBlueprintResources/StandardMacros.DoOnce` false
          (:`Completed`
            (`GameplayStatics.PlaySoundAtLocation` "/Game/Prototype/Sound/Keys/Fence_Opening.Fence_Opening" (`self.K2_GetActorLocation`) (struct) 1.0 1.0 0.0 null null null null)))))))

(event `self.Door Collision.OnComponentBeginOverlap`
  (params (OverlappedComponent :type "PrimitiveComponent Object Reference") (OtherActor :type "Actor Object Reference") (OtherComp :type "PrimitiveComponent Object Reference") (OtherBodyIndex :type Integer) (bFromSweep :type Boolean) (SweepResult :type "HitResult Structure (by ref)"))
  (bind _asbp_player (cast `/Game/Prototype/Test_Player/BP_Player` OtherActor))
  (for (_array_element _array_index) (`self.RequiredKeys`)
    (bind _keyinventory (`/Game/Prototype/Test_Player/BP_Player.KeyInventory` _asbp_player))
    (if (and (`KismetArrayLibrary.Array_Contains` _keyinventory _array_element) (`KismetArrayLibrary.Array_Contains` _keyinventory _array_index))
      (set `self.HasAllKeys` true)
      (if (`self.HasAllKeys`)
        (set `self.IsOpen` true)
        (`KismetSystemLibrary.PrintString` "You have all the keys"))
      (else
        (set `self.HasAllKeys` false)
        (`KismetSystemLibrary.PrintString` "No Keys bruh")
        (for _array_element_2 (`/Game/Prototype/Test_Player/BP_Player.KeyInventory` _asbp_player)
          (`KismetSystemLibrary.PrintString` (`KismetStringLibrary.Conv_IntToString` _array_element_2)))))))

(event `self.Door Collision.OnComponentEndOverlap`
  (params (OverlappedComponent :type "PrimitiveComponent Object Reference") (OtherActor :type "Actor Object Reference") (OtherComp :type "PrimitiveComponent Object Reference") (OtherBodyIndex :type Integer)))

(fn `UserConstructionScript`)