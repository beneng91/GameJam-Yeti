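; Prototype Yeti enemy character that patrols and performs a lethal attack on the player.
; Attack plays a montage and, whether it completes or is interrupted, calls Death on player 0's BP_Player without a hit or range check, then fires OnAttackEnd.
; GetPatrolRoute exposes the assigned route, and SetMovementSpeed maps idle, walking, jogging and running states to max walk speed.
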(event `Attack`
  (`|PlayMontage` (`self.Mesh`) "/Game/Prototype/Test_Yeti/Montage_Attack.Montage_Attack"
    (:`OnCompleted`
      _)
    (:`OnInterrupted`
      _))
  (bind _asbp_player (cast `/Game/Prototype/Test_Player/BP_Player` (`GameplayStatics.GetPlayerCharacter` 0)))
  (`/Game/Prototype/Test_Player/BP_Player.Death` _asbp_player)
  (`self.OnAttackEnd`))

(fn `GetPatrolRoute`
  (returns (PatrolRoute :type "/Game/Prototype/Test_Yeti/AI/BP_PatrolRoute Object Reference"))
  (return (`self.PatrolRoute`)))

(fn `SetMovementSpeed`
  (params (Speed :type "/Game/Prototype/Test_Yeti/AI/Enums/E_MovementSpeed Enum" :default "NewEnumerator0"))
  (returns (SpeedValue :type "Float (double-precision)"))
  (bind _output_get (set `CharacterMovementComponent.MaxWalkSpeed` (select `/Game/Prototype/Test_Yeti/AI/Enums/E_MovementSpeed` Speed :`NewEnumerator1` 200.0 :`NewEnumerator2` 500.0 :`NewEnumerator3` 350.0 :!type "Float (single-precision)") (`self.CharacterMovement`)))
  (return _output_get))

(fn `UserConstructionScript`)